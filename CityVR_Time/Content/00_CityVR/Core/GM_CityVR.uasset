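; GM_CityVR is the game mode for CityVR, spawning and possessing the player's pawn at a chosen player start.
; On BeginPlay it finds the BP_PlayerStart matching the game instance's start number, copying its transform and play-as-PC flag into the VR player settings.
; That flag selects a PC testing pawn or the motion controller VR pawn.
; If the spawned pawn is a BPP_Pawn_CityVR, it receives those settings.
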(event `SpawnPawnToMap`
  (bind _returnvalue (`GameplayStatics.GetPlayerController` 0))
  (bind ((`TestingMode_1_BB7000734920A4149FEE47B97229DFAD` _testingmode) (`SpawnTransform_21_B51524844002F6C672FBF2AD79F84034` _spawntransform)) (break `/Game/00_CityVR/Dev/Structs/Struc_VrPlayerSettings` (`/Game/00_CityVR/Core/GI_CityVr.Struct_VRPlayerSetting` (`self.GameInstance`))))
  (bind _aspawn (castclass `Pawn` (`KismetMathLibrary.SelectClass` "/Game/00_CityVR/Characters/PCPawn/BPC_PCPawn.BPC_PCPawn_C" "/Game/00_CityVR/Characters/VRPawn/MotionControllerPawn_CityVR.MotionControllerPawn_CityVR_C" _testingmode)))
  (bind _returnvalue_2 (`|SpawnActorFromClass` _aspawn _spawntransform "AlwaysSpawn" "OverrideRootScale" _returnvalue null))
  (`Controller.Possess` _returnvalue _returnvalue_2)
  (bind _asbpp_pawn_city_vr (cast `/Game/00_CityVR/Characters/ParentPawn/BPP_Pawn_CityVR` _returnvalue_2))
  (set `/Game/00_CityVR/Characters/ParentPawn/BPP_Pawn_CityVR.Struc_VRPlayerSettings` (`/Game/00_CityVR/Core/GI_CityVr.Struct_VRPlayerSetting` (`self.GameInstance`)) _asbpp_pawn_city_vr))

(event `GetPlayerStartData`
  (for _array_element (`self.BP_Player_Start`)
    (if (== (`/Game/00_CityVR/Dev/BP_PlayerStart.StartNumber` _array_element) (`.PlayerStartNumber_20_989AABCA4A0CB20FE57713B924BA4CAB` (break `/Game/00_CityVR/Dev/Structs/Struc_VrPlayerSettings` (`/Game/00_CityVR/Core/GI_CityVr.Struct_VRPlayerSetting` (`self.GameInstance`)))))
      (setmembers `/Game/00_CityVR/Dev/Structs/Struc_VrPlayerSettings` :`StructRef` (`/Game/00_CityVR/Core/GI_CityVr.Struct_VRPlayerSetting` (`self.GameInstance`)) :`Testing Mode` (`/Game/00_CityVR/Dev/BP_PlayerStart.PlayAsPC` _array_element) :`Spawn Transform` (`self.GetTransform` _array_element)))))

(event `self.ReceiveBeginPlay`
  (bind _asgi_city_vr (cast `/Game/00_CityVR/Core/GI_CityVr` (`GameplayStatics.GetGameInstance`)))
  ;[1 1 1] Get a reference to Game Instance
  (set `self.GameInstance` _asgi_city_vr)
  ;[1 1 1] Get a refenrece to all Player Start
  (bind _outactors (`GameplayStatics.GetAllActorsOfClass` "/Game/00_CityVR/Dev/BP_PlayerStart.BP_PlayerStart_C"))
  (set `self.BP_Player_Start` _outactors)
  (`self.GetPlayerStartData`)
  (`self.SpawnPawnToMap`))

(fn `UserConstructionScript`)